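; Assault rifle weapon Blueprint for the player, with single or automatic fire, timed reload and ammo state saved to the character on unequip.
; Auto fire loops through a Gate and retriggerable delay until StopFiring closes it.
; Each shot uses ammo, line-traces from the camera with random spread, spawns an impact decal and occasional tracer, then triggers animations and muzzle flash.
; Hits apply no damage, and the second muzzle-to-impact trace's result is unused.
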(event EventUnequip
  ;[1 1 1] Unequip
  (Variables|/Game/Blueprints/BP_FemaleCharacterBase.BP_FemaleCharacterBase_C|SetprimaryWeapon (Utilities|CasttoPlayer) (Utilities|Struct|MakeGunData "NewEnumerator1" "AR_Weapon_C" (Variables|Default|GetammoCount) (Variables|Default|GetmaxAmmo) (Variables|Default|GetreloadTime) (Variables|Default|GetbulletSpread))))

(event EventStopFiring
  ;[1 1 1] Handle Auto Fire
  (Utilities|FlowControl|Gate true) ; enters at Close
)

(event EventFire
  ;[1 1 1] Toggle Single/Auto Fire
  (if (Variables|Default|GetsingleFire)
    _
    (else
      ;[1 1 1] Handle Auto Fire
      (Utilities|FlowControl|Sequence
        (:then_0
          (goto _label Open))
        (:then_1
          (Utilities|FlowControl|Gate true :!label _label
            (:Exit
              (Utilities|FlowControl|Sequence
                (:then_0
                  _)
                (:then_1
                  (Utilities|FlowControl|RetriggerableDelay 0.12)
                  (goto _label)))))))))
  (if (> (Variables|Default|GetammoCount) 0)
    (CallFunction|AmmoCheck)
    (bind (_impactpoint _muzzleloc) (CallFunction|ShootTrace))
    (CallFunction|SpawnDecal _impactpoint _impactpoint _muzzleloc)
    (Animation|Montage|PlayMontage (Variables|/Script/Engine.Character|GetMesh (Utilities|CasttoPlayer)) 0 ; Player Shoot Animation here
      (:then
        (Utilities|MuzzleFlash)))
    (else
      (Audio|PlaySoundatLocation "/Game/Assets/Audio/dryFire.dryFire" (Utilities|GetCameraLocation) "0, 0, 0" 1.0 1.0 0.0 0 0 0))))

(event EventReload
  (bind _asbp_female_character_base (Utilities|CasttoPlayer))
  ;[1 1 1] Reload
  (if (< (Variables|Default|GetammoCount) (Variables|Default|GetmaxAmmo))
    (Utilities|FlowControl|DoOnce false :!label _label
      (:Completed
        (Variables|/Game/Blueprints/BP_FemaleCharacterBase.BP_FemaleCharacterBase_C|SetisReloading _asbp_female_character_base true)
        (Animation|Montage|MontagePlay (Components|SkeletalMesh|GetAnimInstance (Variables|/Script/Engine.Character|GetMesh _asbp_female_character_base)) 0 1.0 "MontageLength" 0.0 true) ; Player reload animation
        (Components|Animation|PlayAnimation (Variables|Default|GetPrimaryWeapon) 0 false) ; Reload Animation Here
        (Utilities|FlowControl|Delay (Variables|Default|GetreloadTime))
        (Variables|Default|SetammoCount (Variables|Default|GetmaxAmmo))
        (Variables|/Game/Blueprints/BP_FemaleCharacterBase.BP_FemaleCharacterBase_C|SetisReloading _asbp_female_character_base false)
        (goto _label Reset)))))

(fn ConstructionScript
  (|CallParentFunction)
  (Variables|Default|SetmaxAmmo 30)
  (Variables|Default|SetammoCount 30)
  (Variables|Default|SetreloadTime 2.0)
  (Variables|Default|SetbulletSpread 2.5e+02)
  (Variables|Default|SetName "NewEnumerator1")
  (Variables|Default|SetvariableMode true))

(fn AmmoCheck
  (bind _returnvalue (Math|Random|RandomFloatinRange 0.7 1.2))
  (Math|Integer|DecrementInt (Variables|Default|GetammoCount)
    (:%20%20
      (Audio|PlaySoundatLocation "/Game/Assets/Audio/pop.pop" (Utilities|GetCameraLocation) "0, 0, 0" (+ _returnvalue 1.0) _returnvalue 0.0 0 0 0)
      (Components|Animation|PlayAnimation (Variables|Default|GetPrimaryWeapon) 0 false) ; Gun Shoot Animation Here
    )))

(fn ShootTrace
  (bind _returnvalue (Game|GetPlayerCharacter 0))
  (bind _muzzle (Variables|Default|GetMuzzle))
  (bind _bulletspread (Variables|Default|GetbulletSpread))
  (bind _returnvalue_2 (Transformation|GetWorldLocation _muzzle))
  (bind _returnvalue_3 (* _bulletspread -0.5))
  (bind _asbp_female_character_base (Utilities|Casting|CastToBP_FemaleCharacterBase _returnvalue))
  (bind _cameracomp (Variables|/Script/ProjectDraft.FemaleCharacterBase|GetCameraComp _asbp_female_character_base))
  (bind _returnvalue_4 (Transformation|GetWorldLocation _cameracomp))
  ;[1 1 1] Linetrace from camera
  (bind _outhit (Collision|LineTraceByChannel _returnvalue_4 (+ (+ _returnvalue_4 (* (Math|Vector|GetForwardVector _cameracomp) 2e+04)) (Math|Vector|MakeVector (Math|Random|RandomFloatinRange _returnvalue_3 _bulletspread) (Math|Random|RandomFloatinRange _returnvalue_3 _bulletspread) (Math|Random|RandomFloatinRange _returnvalue_3 _bulletspread))) "TraceTypeQuery1" false 0 "None")) ; Camera Shot
  (Collision|LineTraceByChannel _returnvalue_2 (.ImpactPoint (Collision|BreakHitResult _outhit)) "TraceTypeQuery1" false 0 "None" true "(R=1.000000,G=0.000000,B=0.855670,A=1.000000)" "(R=0.000000,G=0.845457,B=1.000000,A=1.000000)") ; Gun Shot
  (return (.ImpactPoint (Collision|BreakHitResult _outhit)) _returnvalue_2))

(fn SpawnDecal
  (params (ImpactPoint :type Vector) (SpawnTransformLoc :type Vector) (Location :type Vector))
  (Game|SpawnActorfromClass "/Game/Blueprints/BP_Decal.BP_Decal_C" (Math|Transform|MakeTransform SpawnTransformLoc (Math|Conversions|RotationFromXVector ImpactPoint) "0.025000,0.025000,0.025000") "Undefined" 0 0)
  (if (>= (Math|Random|RandomIntegerinRange 1 10) 5)
    (Game|SpawnActorfromClass "/Game/Blueprints/BP_TracerRounds.BP_TracerRounds_C" (Math|Transform|MakeTransform Location (Transformation|GetWorldRotation (Utilities|GetCamera))) "Undefined" 0 0))
  (return))