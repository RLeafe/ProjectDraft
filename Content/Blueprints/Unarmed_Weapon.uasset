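; Unarmed weapon Blueprint that sets its name enum and disables VariableMode on construction, yet carries gun-firing functions.
; ShootTrace traces from the player camera with random spread, traces from muzzle to that hit, and returns impact and muzzle locations.
; AmmoCheck decrements ammo and plays randomized shot audio and animation.
; SpawnDecal places a decal plus occasional tracer, while MuzzleFlash pulses a light and randomized plane.
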(fn ConstructionScript
  (|CallParentFunction)
  (Variables|Default|SetName "NewEnumerator0")
  (Variables|Default|SetvariableMode false))

(fn AmmoCheck
  (bind _returnvalue (Math|Random|RandomFloatinRange 0.7 1.2))
  (Math|Integer|DecrementInt (Variables|Default|GetammoCount)
    (:%20%20
      (Audio|PlaySoundatLocation "/Game/Assets/Audio/pop.pop" (Utilities|GetCameraLocation) "0, 0, 0" (+ _returnvalue 1.0) _returnvalue 0.0 0 0 0)
      (Components|Animation|PlayAnimation (Variables|Default|GetPrimaryWeapon) 0 false) ; Gun Shoot Animation Here
    )))

(fn ShootTrace
  (bind _returnvalue (Game|GetPlayerCharacter 0))
  (bind _muzzle (Variables|Default|GetMuzzle))
  (bind _bulletspread (Variables|Default|GetbulletSpread))
  (bind _returnvalue_2 (Transformation|GetWorldLocation _muzzle))
  (bind _returnvalue_3 (* _bulletspread -0.5))
  (bind _asbp_female_character_base (Utilities|Casting|CastToBP_FemaleCharacterBase _returnvalue))
  (bind _cameracomp (Variables|/Script/ProjectDraft.FemaleCharacterBase|GetCameraComp _asbp_female_character_base))
  (bind _returnvalue_4 (Transformation|GetWorldLocation _cameracomp))
  ;[1 1 1] Linetrace from camera
  (bind _outhit (Collision|LineTraceByChannel _returnvalue_4 (+ (+ _returnvalue_4 (* (Math|Vector|GetForwardVector _cameracomp) 2e+04)) (Math|Vector|MakeVector (Math|Random|RandomFloatinRange _returnvalue_3 _bulletspread) (Math|Random|RandomFloatinRange _returnvalue_3 _bulletspread) (Math|Random|RandomFloatinRange _returnvalue_3 _bulletspread))) "TraceTypeQuery1" false 0 "None")) ; Camera Shot
  (Collision|LineTraceByChannel _returnvalue_2 (.ImpactPoint (Collision|BreakHitResult _outhit)) "TraceTypeQuery1" false 0 "None" true "(R=1.000000,G=0.000000,B=0.855670,A=1.000000)" "(R=0.000000,G=0.845457,B=1.000000,A=1.000000)") ; Gun Shot
  (return (.ImpactPoint (Collision|BreakHitResult _outhit)) _returnvalue_2))

(fn SpawnDecal
  (params (ImpactPoint :type Vector) (SpawnTransformLoc :type Vector) (Location :type Vector))
  (Game|SpawnActorfromClass "/Game/Blueprints/BP_Decal.BP_Decal_C" (Math|Transform|MakeTransform SpawnTransformLoc (Math|Conversions|RotationFromXVector ImpactPoint) "0.025000,0.025000,0.025000") "Undefined" 0 0)
  (if (>= (Math|Random|RandomIntegerinRange 1 10) 5)
    (Game|SpawnActorfromClass "/Game/Blueprints/BP_TracerRounds.BP_TracerRounds_C" (Math|Transform|MakeTransform Location (Transformation|GetWorldRotation (Utilities|GetCamera))) "Undefined" 0 0))
  (return))